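; Inventory component that stores items in a fixed number of slots and toggles the inventory window on the HUD canvas.
; Slots are resized and their item info refreshed from class defaults on BeginPlay and each time the window opens.
; Adding tops up partial stacks, recursively re-adding overflow, or fills an empty slot.
; Helpers subtract amounts from slots and check whether total holdings of an item class meet a required quantity.
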(event `self.ReceiveBeginPlay`
  (`self.prepareInventory`))

(fn `addToInventory`
  (params (contentToAdd :type "/Game/InventorySystem/Widgets/S_SlotStructure Structure"))
  (returns (`succsess?` :type Boolean))
  (if (`.isStackable_12_95ED1C244D16A774458FC38CC75FAB5A` (break `/Game/InventorySystem/Blueprint/S_ItemInfo` (break `/Game/InventorySystem/Widgets/S_SlotStructure` contentToAdd)))
    (bind _stackindex (`self.hasPartialStack` (`local.contentToAdd`))
      (:`true`
        (`self.addToStack` (`local.contentToAdd`) _stackindex)
        (return true))
      (:`false`
        _)))
  (`self.createStack` (`local.contentToAdd`))
  (return true))

(fn `addToStack`
  (params (slotStructure :type "/Game/InventorySystem/Widgets/S_SlotStructure Structure") (slotIndex :type Integer))
  (returns (succsess :type Boolean))
  (locals (currentAmount :type Integer))
  (bind _slotindex (`local.slotIndex`))
  (bind _inventory (`self.Inventory`))
  (bind (_slotstructure_itemstructure _slotstructure_amount) (break `/Game/InventorySystem/Widgets/S_SlotStructure` (`local.slotStructure`)))
  (bind _slotstructure_itemstructure_2 (break `/Game/InventorySystem/Widgets/S_SlotStructure` (`local.slotStructure`)))
  (bind (_slotstructure_itemstructure_3 _slotstructure_amount_2) (break `/Game/InventorySystem/Widgets/S_SlotStructure` (`local.slotStructure`)))
  (bind (_name _description _image _isusable _isstackable _category _class _maxstacksize) (break `/Game/InventorySystem/Blueprint/S_ItemInfo` _slotstructure_itemstructure_2))
  (bind _output (`|GetArrayItem` (`self.Inventory`) slotIndex))
  (bind (_output_itemstructure _output_amount) (break `/Game/InventorySystem/Widgets/S_SlotStructure` (`|GetArrayItem` _inventory _slotindex)))
  (bind _output_get (set `local.currentAmount` (`.Amount_5_D68E1E46435A98CB719B63836D306992` (break `/Game/InventorySystem/Widgets/S_SlotStructure` _output))))
  (if (> (+ _output_get (`.Amount_5_D68E1E46435A98CB719B63836D306992` (break `/Game/InventorySystem/Widgets/S_SlotStructure` slotStructure))) (`.maxStackSIze_22_9BF1532348B981E67D6F92885C9C99D2` (break `/Game/InventorySystem/Blueprint/S_ItemInfo` (break `/Game/InventorySystem/Widgets/S_SlotStructure` _output))))
    (`KismetArrayLibrary.Array_Set` (`self.Inventory`) (`local.slotIndex`) (make `/Game/InventorySystem/Widgets/S_SlotStructure` _slotstructure_itemstructure_2 _maxstacksize))
    (bind _succsess_ (`self.addToInventory` (make `/Game/InventorySystem/Widgets/S_SlotStructure` _slotstructure_itemstructure_3 (- _slotstructure_amount_2 (- _maxstacksize (`local.currentAmount`))))))
    (else
      (`KismetArrayLibrary.Array_Set` _inventory _slotindex (make `/Game/InventorySystem/Widgets/S_SlotStructure` _output_itemstructure (+ _output_amount _slotstructure_amount)))))
  (return _succsess_))

(fn `createStack`
  (params (contentToAdd :type "/Game/InventorySystem/Widgets/S_SlotStructure Structure"))
  (returns (succsess :type Boolean))
  (locals (hasSpace :type Boolean))
  (bind _inventory (`self.Inventory`))
  (for _array_element (`self.Inventory`)
    (if (<= (`.Amount_5_D68E1E46435A98CB719B63836D306992` (break `/Game/InventorySystem/Widgets/S_SlotStructure` _array_element)) 0)
      (set `local.hasSpace` true)
      (break)))
  (if (`local.hasSpace`)
    (`KismetArrayLibrary.Array_Set` _inventory (`KismetArrayLibrary.Array_Find` _inventory (make `/Game/InventorySystem/Widgets/S_SlotStructure` (struct :`Category` "NewEnumerator0" :`maxStackSIze` 99 :`ArmorData` (struct :`ArmorType` "NewEnumerator0" :`Rarity` "NewEnumerator0")))) (`local.contentToAdd`))
    (return (`local.hasSpace`))
    (else
      (return false))))

(fn `inventoryQuery`
  (params (QueryItem :type "/Game/InventorySystem/Items/Item Class Reference") (queryAmount :type Integer))
  (returns (isInInventory :type Boolean))
  (locals (_succsess :type Boolean) (_runningTotal :type Integer))
  (for _array_element (`self.Inventory`)
    (if (== (`local.QueryItem`) (`.Class_18_D3172BBF4A0C9DF7C58341ACA4E48CA2` (break `/Game/InventorySystem/Blueprint/S_ItemInfo` (break `/Game/InventorySystem/Widgets/S_SlotStructure` _array_element))))
      (set `local._runningTotal` (+ (`.Amount_5_D68E1E46435A98CB719B63836D306992` (break `/Game/InventorySystem/Widgets/S_SlotStructure` _array_element)) (`local._runningTotal`)))))
  (return (>= (`local._runningTotal`) (`local.queryAmount`))))

(fn `prepareInventory`
  (`KismetArrayLibrary.Array_Resize` (`self.Inventory`) (`self.numberOfSlots`))
  (for (_array_element _array_index) (`self.Inventory`)
    (bind (_name _description _image _isusable _isstackable _category _class) (break `/Game/InventorySystem/Blueprint/S_ItemInfo` (break `/Game/InventorySystem/Widgets/S_SlotStructure` _array_element)))
    (if (!= _class null)
      (`KismetArrayLibrary.Array_Set` (`self.Inventory`) _array_index (make `/Game/InventorySystem/Widgets/S_SlotStructure` (defaults `/Game/InventorySystem/Blueprint/InventoryComponent` _class) (`.Amount_5_D68E1E46435A98CB719B63836D306992` (break `/Game/InventorySystem/Widgets/S_SlotStructure` _array_element)))))))

(fn `removeItem`
  (params (SlotStructure :type "/Game/InventorySystem/Widgets/S_SlotStructure Structure") (amount :type Integer))
  (returns (succsess :type Boolean))
  (locals (_index :type Integer :default 0) (_amount :type Integer))
  (set `local._amount` amount)
  (bind _output_get (set `local._index` (`KismetArrayLibrary.Array_Find` (`self.Inventory`) SlotStructure)))
  (bind (_output_itemstructure _output_amount) (break `/Game/InventorySystem/Widgets/S_SlotStructure` (`|GetArrayItem` (`self.Inventory`) _output_get)))
  (bind _returnvalue (- _output_amount (`local._amount`)))
  (if (>= _returnvalue 0)
    (`KismetArrayLibrary.Array_Set` (`self.Inventory`) (`local._index`) (make `/Game/InventorySystem/Widgets/S_SlotStructure` _output_itemstructure _returnvalue))
    (return true)
    (elif (== _returnvalue 0)
      (`KismetArrayLibrary.Array_Set` (`self.Inventory`) (`local._index`) (make `/Game/InventorySystem/Widgets/S_SlotStructure` (struct :`Category` "NewEnumerator0" :`maxStackSIze` 99 :`ArmorData` (struct :`ArmorType` "NewEnumerator0" :`Rarity` "NewEnumerator0"))))
      (return true)
      (else
        (return false)))))

(fn `toggleInventory`
  (bind _returnvalue (`GameplayStatics.GetPlayerController` 0))
  (bind (_anchors_minimum _anchors_maximum) (break `Anchors` (`self.anchors`)))
  (`self.InventoryWindow`
    (:`then`
      (`Widget.RemoveFromParent` (`self.InventoryWindow`))
      (set `self.InventoryWindow` null)
      (`WidgetBlueprintLibrary.SetInputMode_GameOnly` _returnvalue)
      (set `PlayerController.bShowMouseCursor` false _returnvalue))
    (:`else`
      (`self.prepareInventory`)
      (bind _returnvalue_2 (`|CreateWidget` "/Game/InventorySystem/Widgets/BP_Inventory.BP_Inventory_C" null self))
      (set `self.InventoryWindow` _returnvalue_2)
      (bind _asbp_player_controller (cast `/Game/ThirdPersonBP/Blueprints/BP_PlayerController` (`GameplayStatics.GetPlayerController` 0)))
      (bind _returnvalue_3 (`CanvasPanel.AddChildToCanvas` (`/Game/ThirdPersonBP/Blueprints/BP_Hud.HudCAnvas` (`/Game/ThirdPersonBP/Blueprints/BP_PlayerController.HudWidget` _asbp_player_controller)) (`self.InventoryWindow`)))
      (`CanvasPanelSlot.SetAutoSize` _returnvalue_3 true)
      (`CanvasPanelSlot.SetAnchors` _returnvalue_3 (`self.anchors`))
      (`CanvasPanelSlot.SetAlignment` _returnvalue_3 _anchors_maximum)
      (`WidgetBlueprintLibrary.SetInputMode_GameAndUIEx` (`GameplayStatics.GetPlayerController` 0) (`self.InventoryWindow`)))))